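; BP_lightning is an effect Blueprint that makes a light flash like lightning at irregular intervals.
; On BeginPlay it plays a timeline whose curve, scaled by Intensity, drives the Lightning component's intensity.
; When the timeline finishes, it waits a base delay plus a random amount from RandomDelayRange, then restarts itself in an endless loop.
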(event Custom|LightningStart
  (bind _randomdelayrange (Variables|Default|GetRandomDelayRange))
  (bind _auschlag (Timeline|Timeline PlayFromStart)
    (:Update
      (Rendering|Components|Light|SetIntensity (Variables|Default|GetLightning) (* _auschlag (Variables|Default|GetIntensity))))
    (:Finished
      (Utilities|FlowControl|Delay (+ (Math|Float|Lerp (.min _randomdelayrange) (.max _randomdelayrange) (Math|Random|RandomFloat)) (Variables|Default|GetBaseDelay)))
      (CallFunction|LightningStart))))

(event EventBeginPlay
  (CallFunction|LightningStart))

(fn ConstructionScript)