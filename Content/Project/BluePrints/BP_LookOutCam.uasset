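; Possessable lookout camera that lets the player look around from a placed viewpoint.
; Look input rotates the camera at a frame-time-scaled rate, flipping pitch sign based on the actor's starting yaw, then passes relative rotation through ClampRotatorCustom with min and max limits.
; Possession resets the camera's relative rotation.
; Interact or Escape hands player 0's controller back to BP_Player1P.
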(event Input|EnhancedActionEvents|EnhancedInputActionIA_Look
  (params (ActionValue :type Vector%202D%20Structure) (ElapsedSeconds :type Float%20%28double-precision%29) (TriggeredSeconds :type Float%20%28double-precision%29) (InputAction :type Input%20Action%20Object%20Reference :default "/Game/FirstPerson/Input/Actions/IA_Look.IA_Look"))
  (bind _returnvalue (Utilities|Time|GetWorldDeltaSeconds))
  (bind _base_turn_rate (Variables|Default|GetBase%20Turn%20Rate))
  (bind _camera (Variables|Default|GetCamera))
  (bind _returnvalue_2 (* (.x ActionValue) _returnvalue _base_turn_rate))
  (bind _returnvalue_3 (* _returnvalue (.y ActionValue) _base_turn_rate))
  ;[1 1 1] Look
  (if (< (.yaw (Variables|Default|GetBaseRotation)) 179.0)
    (Transformation|AddWorldRotation _camera (Math|Rotator|MakeRotator 0.0 (* _returnvalue_3 -1.0) _returnvalue_2) false false)
    (else
      (Transformation|AddWorldRotation _camera (Math|Rotator|MakeRotator 0.0 _returnvalue_3 _returnvalue_2) false false)))
  (Transformation|SetRelativeRotation _camera (Utilities|ClampRotatorCustom (Variables|/Script/Engine.SceneComponent|GetRelativeRotation _camera) (Variables|Default|GetRotationMin) (Variables|Default|GetRotationMax)) false false))

(event Input|EnhancedActionEvents|EnhancedInputActionIA_Interact
  (params (ActionValue :type Boolean) (ElapsedSeconds :type Float%20%28double-precision%29) (TriggeredSeconds :type Float%20%28double-precision%29) (InputAction :type Input%20Action%20Object%20Reference :default "/Game/FirstPerson/Input/Actions/IA_Interact.IA_Interact"))
  ;[1 1 1] EXIT Cam
  (bind _returnvalue (Actor|GetActorOfClass "/Game/Project/BluePrints/BP_Player1P.BP_Player1P_C"))
  (Pawn|Possess (Game|GetPlayerController 0) _returnvalue))

(event Input|EnhancedActionEvents|EnhancedInputActionIA_ESC
  (params (ActionValue :type Boolean) (ElapsedSeconds :type Float%20%28double-precision%29) (TriggeredSeconds :type Float%20%28double-precision%29) (InputAction :type Input%20Action%20Object%20Reference :default "/Game/FirstPerson/Input/Actions/IA_ESC.IA_ESC"))
  ;[1 1 1] EXIT Cam
  (bind _returnvalue (Actor|GetActorOfClass "/Game/Project/BluePrints/BP_Player1P.BP_Player1P_C"))
  (Pawn|Possess (Game|GetPlayerController 0) _returnvalue))

(event EventPossessed
  (params (NewController :type Controller%20Object%20Reference))
  ;[1 1 1] On Possess
  (Transformation|SetRelativeRotation (Variables|Default|GetCamera) "0, 0, 0" false false))

(event EventBeginPlay
  ;[1 1 1] On Begin
  (Variables|Default|SetBaseRotation (Transformation|GetActorRotation)))

(fn ConstructionScript)