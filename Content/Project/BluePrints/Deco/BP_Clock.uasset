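; BP_Clock is a decorative wall clock whose hands show a stored time and can optionally run during play.
; When RunClock enables Tick, seconds advance by ClockSpeed and carry into minutes, with minute rollover setting the hour to 1.
; SecondPointerOnly stops that carry and removes the hour hand's minute-based offset.
; SetPointers turns the time into hand pitch rotations each tick and in the Construction Script, so the set time shows in the editor.
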(event EventTick
  (params (DeltaSeconds :type Float%20%28single-precision%29))
  (Utilities|FlowControl|Sequence
    (:then_0
      (bind _structout (Utilities|Struct|SetmembersinS_ClockTime (Variables|Clock|GetTime) (+ (* DeltaSeconds (Variables|Clock|GetClockSpeed)) (.second (Variables|Clock|GetTime)))))
      (if (Variables|Clock|GetSecondPointerOnly)
        (if (>= (.Second (Utilities|Struct|BreakS_ClockTime _structout)) 6e+01)
          (Utilities|Struct|SetmembersinS_ClockTime _structout 0.0))
        (elif (>= (.Second (Utilities|Struct|BreakS_ClockTime _structout)) 6e+01)
          (bind _structout_2 (Utilities|Struct|SetmembersinS_ClockTime _structout (+ (.Minutes (Utilities|Struct|BreakS_ClockTime _structout)) 1) 0.0))
          (if (>= (.Minutes (Utilities|Struct|BreakS_ClockTime _structout_2)) 6e+01)
            (bind _structout_3 (Utilities|Struct|SetmembersinS_ClockTime _structout_2 (+ 0 1)))
            (if (>= (.Hour (Utilities|Struct|BreakS_ClockTime _structout_3)) 12)
              (Utilities|Struct|SetmembersinS_ClockTime _structout_3))))))
    (:then_1
      (CallFunction|SetPointers))))

(event EventBeginPlay
  (Actor|Tick|SetActorTickEnabled (Variables|Clock|GetRunClock)))

(fn ConstructionScript
  (CallFunction|SetPointers))

(fn SetPointers
  (bind _returnvalue (/ 0.0 1e+01))
  (bind _time (Variables|Clock|GetTime))
  (bind _wallclock_lp_minutes_pointer (Variables|Default|GetWallClock_LP_Minutes_Pointer))
  (bind _wallclock_lp_hours_pointer (Variables|Default|GetWallClock_LP_Hours_Pointer))
  (bind _time_2 (Variables|Clock|GetTime))
  (bind _returnvalue_2 (* (.minutes _time_2) 6))
  (bind _returnvalue_3 (+ _returnvalue_2 _returnvalue))
  (Transformation|SetRelativeRotation (Variables|Default|GetWallClock_LP_Seconds_Pointer) (Math|Rotator|MakeRotator 0.0 (* (* (.second _time_2) 6.0) -1.0) 0.0) false false)
  (if (Variables|Clock|GetSecondPointerOnly)
    (Transformation|SetRelativeRotation _wallclock_lp_minutes_pointer (Math|Rotator|MakeRotator 0.0 (* (* (.minutes _time) 6) -1.0) 0.0) false false)
    (Transformation|SetRelativeRotation _wallclock_lp_hours_pointer (Math|Rotator|MakeRotator 0.0 (* (* (.hour _time) 30) -1.0) 0.0) false false)
    (else
      (Transformation|SetRelativeRotation _wallclock_lp_minutes_pointer (Math|Rotator|MakeRotator 0.0 (* _returnvalue_3 -1.0) 0.0) false false)
      (Transformation|SetRelativeRotation _wallclock_lp_hours_pointer (Math|Rotator|MakeRotator 0.0 (* (+ (* (.hour _time_2) 30) (/ _returnvalue_3 12.0)) -1.0) 0.0) false false))))