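; Horror event receiver Blueprint that starts and stops a horror event after a given delay, guarded by an IsActive flag.
; Triggering, including via ManualTrigger, cascades to dependent event actors with their own start delays and stretches EventDuration to cover the longest.
; OnEventStart schedules the stop after that duration when StopAfterDuration is set.
; OnEventStop is an empty hook, and stopping does not propagate to dependents.
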(event Custom|ManualTrigger
  (CallFunction|TriggertheHorrorEvent 0.0))

(event EventTriggertheHorrorEvent
  (params (Delay :type Float%20%28double-precision%29))
  (bind _dependenthorrorevents (Variables|HorrorEventReciever|GetDependentHorrorEvents))
  ;[1 1 1] Start
  (Utilities|FlowControl|Delay Delay)
  (if (not (Variables|HorrorEventReciever|GetIsActive))
    (Variables|HorrorEventReciever|SetIsActive true)
    (Utilities|FlowControl|Sequence
      (:then_0
        (if (Utilities|Array|IsNotEmpty _dependenthorrorevents)
          (for _array_element _dependenthorrorevents
            (Default|TriggertheHorrorEvent (.horroreventactor _array_element) (.delaystart _array_element))
            (if (> (+ (.delaystart _array_element) (Variables|BP_HorrorEventReciever_C|GetEventDuration (.horroreventactor _array_element))) (Variables|HorrorEventReciever|GetEventDuration))
              (Variables|HorrorEventReciever|SetEventDuration (+ (.delaystart _array_element) (Variables|BP_HorrorEventReciever_C|GetEventDuration (.horroreventactor _array_element))))))))
      (:then_1
        (CallFunction|OnEventStart)))))

(event EventStoptheHorrorEvent
  (params (Delay :type Float%20%28double-precision%29))
  ;[1 1 1] Stop
  (Utilities|FlowControl|Delay Delay)
  (if (Variables|HorrorEventReciever|GetIsActive)
    (Variables|HorrorEventReciever|SetIsActive false)
    (CallFunction|OnEventStop)))

(fn ConstructionScript)

(fn OnEventStart
  (if (Variables|HorrorEventReciever|GetStopAfterDuration)
    (CallFunction|StoptheHorrorEvent (Variables|HorrorEventReciever|GetEventDuration))))

(fn OnEventStop)