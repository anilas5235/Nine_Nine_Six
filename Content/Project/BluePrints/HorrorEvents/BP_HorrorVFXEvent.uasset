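; BP_HorrorVFXEvent is a horror event Blueprint that switches a visual effect component on and off with the event's lifecycle.
; The Effect component is deactivated at BeginPlay, activated with a reset when the event starts, and deactivated when it stops.
; The start and stop overrides call their parent implementations after toggling the effect.
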(event EventBeginPlay
  (Components|Activation|Deactivate (Variables|Default|GetEffect)))

(fn ConstructionScript
  (|CallParentFunction))

(fn OnEventStart
  (Components|Activation|Activate (Variables|Default|GetEffect) true)
  (|CallParentFunction))

(fn OnEventStop
  (Components|Activation|Deactivate (Variables|Default|GetEffect))
  (|CallParentFunction))