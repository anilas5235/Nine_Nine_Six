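; BP_AnormalyHandler is an actor that manages a group of dependent horror events for an anomaly.
; On BeginPlay it registers itself in the AnormalyHandlers array of the object returned by TryGetPC996.
; OnEventStop loops over DependentHorrorEvents and immediately calls StopTheHorrorEvent on each entry's horror event actor.
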(event EventBeginPlay
  (|CallParentFunction)
  (bind _aspc_996 (CallFunction|TryGetPC996))
  (Utilities|Array|Add (Variables|/Game/Project/Managers/PC_996.PC_996_C|GetAnormalyHandlers _aspc_996) self))

(fn ConstructionScript
  (|CallParentFunction))

(fn OnEventStop
  (for _array_element (Variables|Default|GetDependentHorrorEvents)
    (Default|StoptheHorrorEvent (.horroreventactor _array_element) 0.0)))