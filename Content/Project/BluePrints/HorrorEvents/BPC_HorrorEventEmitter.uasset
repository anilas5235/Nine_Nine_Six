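; BPC_HorrorEventEmitter is a component that triggers one of its horror event relays at random, either on demand or after a random delay.
; StartNextTimer schedules a single Fire within the delay bounds when relays exist, and StopCurrentTimer cancels it.
; Fire picks a new index based on the last one, triggers that relay and prints the index.
; Fire does not reschedule itself, so each timed event needs another StartNextTimer call.
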(event Custom|Fire
  (bind _horroreventrelays (Variables|HorrorEventEmitter|GetHorrorEventRelays))
  ;[1 1 1] Timer
  (bind (_index _isnew _isvaild) (CallFunction|TryGetNewRandomIndex (Variables|HorrorEventEmitter|GetLastIndex) (Utilities|Array|Length _horroreventrelays)))
  (if _isvaild
    (bind _output_get (Variables|HorrorEventEmitter|SetLastIndex _index))
    (Default|TriggerHorrorEventRelay (Utilities|Array|Get(acopy) _horroreventrelays _index))
    (Development|PrintString (Utilities|String|Append "To Relay:" (Utilities|String|ToString(Integer) _output_get)))))

(event Custom|StartNextTimer
  (bind _randomdelaybounds (Variables|HorrorEventEmitter|GetRandomDelayBounds))
  ;[1 1 1] Timer
  (if (Utilities|Array|IsNotEmpty (Variables|HorrorEventEmitter|GetHorrorEventRelays))
    (bind _returnvalue (Utilities|Time|SetTimerbyEvent (delegate Custom|Fire) (Math|Random|RandomFloatinRange (.min _randomdelaybounds) (.max _randomdelaybounds))))
    (Variables|HorrorEventEmitter|SetCurrentTimer _returnvalue)))

(event Custom|StopCurrentTimer
  ;[1 1 1] Cancel Timer
  (if (Utilities|Time|IsValidTimerHandle (Variables|HorrorEventEmitter|GetCurrentTimer))
    (Utilities|Time|ClearandInvalidateTimerbyHandle (Variables|HorrorEventEmitter|GetCurrentTimer))))

(event Custom|ManualFire
  ;[1 1 1] Manual
  (CallFunction|Fire))