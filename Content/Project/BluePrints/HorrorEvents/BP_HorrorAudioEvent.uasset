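; BP_HorrorAudioEvent is a horror event that plays the sound assigned to its Audio component.
; OnEventStart plays the sound or prints an error naming the Blueprint when none is set.
; With StopAfterDuration enabled, it passes EventDuration, or the sound's own length when that is zero, to StopTheHorrorEvent.
; OnEventStop stops the audio and also runs on BeginPlay to keep it silent initially.
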(event EventBeginPlay
  (CallFunction|OnEventStop))

(fn ConstructionScript
  (|CallParentFunction))

(fn OnEventStart
  (bind _audio (Variables|Default|GetAudio))
  (bind _eventduration (Variables|Default|GetEventDuration))
  (bind _sound (Variables|/Script/Engine.AudioComponent|GetSound _audio))
  (Utilities|IsValid _sound
    (:Is%20Valid
      (Audio|Components|Audio|Play _audio 0.0)
      (if (Variables|Default|GetStopAfterDuration)
        (if (== 0.0 _eventduration)
          (CallFunction|StoptheHorrorEvent (Variables|/Script/Engine.SoundBase|GetDuration _sound))
          (else
            (CallFunction|StoptheHorrorEvent _eventduration)))))
    (:Is%20Not%20Valid
      (Development|PrintString (Utilities|String|Append "Sound not set in" (Utilities|GetDisplayName self))))))

(fn OnEventStop
  (Audio|Components|Audio|Stop (Variables|Default|GetAudio)))