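; BP_HorrorDecalEvent is a horror event that reveals a decal and plays a sound when triggered.
; OnEventStart makes the referenced Decal actor's root component visible, starts the audio and then calls the parent implementation.
; OnEventStop hides the decal and stops the audio without calling the parent, and also runs on BeginPlay so the event starts hidden and silent.
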(event EventBeginPlay
  (CallFunction|OnEventStop))

(fn ConstructionScript
  (|CallParentFunction))

(fn OnEventStart
  (bind _decal (Variables|Default|GetDecal))
  (Utilities|IsValid _decal
    (:Is%20Valid
      (Rendering|SetVisibility (Variables|/Script/Engine.Actor|GetRootComponent _decal) true false))
    (:Is%20Not%20Valid
      _))
  (Audio|Components|Audio|Play (Variables|Default|GetAudio) 0.0)
  (|CallParentFunction))

(fn OnEventStop
  (bind _decal (Variables|Default|GetDecal))
  (Utilities|IsValid _decal
    (:Is%20Valid
      (Rendering|SetVisibility (Variables|/Script/Engine.Actor|GetRootComponent _decal) false false))
    (:Is%20Not%20Valid
      _))
  (Audio|Components|Audio|Stop (Variables|Default|GetAudio)))