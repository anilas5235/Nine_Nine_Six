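; Horror event Blueprint that reveals an animated skeletal mesh actor while the event runs.
; The actor hides itself on BeginPlay and waits for the event hooks inherited from its parent class.
; OnEventStart unhides it and plays the mesh animation once without looping, and OnEventStop hides it again.
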(event EventBeginPlay
  (Rendering|SetActorHiddenInGame true))

(fn ConstructionScript
  (|CallParentFunction))

(fn OnEventStart
  (|CallParentFunction)
  (Rendering|SetActorHiddenInGame false)
  (Audio|Components|Audio|Play (Variables|Default|GetSkeletalMesh) false))

(fn OnEventStop
  (|CallParentFunction)
  (Rendering|SetActorHiddenInGame true))