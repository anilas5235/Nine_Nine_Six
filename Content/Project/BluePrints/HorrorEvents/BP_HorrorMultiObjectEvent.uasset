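; BP_HorrorMultiObjectEvent is a horror event that temporarily shows a group of actors.
; It hides every actor in DependentVisualActors on BeginPlay by calling OnEventStop.
; OnEventStart unhides them all and passes EventDuration to StopTheHorrorEvent, while OnEventStop hides them again.
; Both handlers do nothing when the actor list is empty, so an empty list also skips the StopTheHorrorEvent call.
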(event EventBeginPlay
  (CallFunction|OnEventStop))

(fn ConstructionScript
  (|CallParentFunction))

(fn OnEventStart
  (bind _dependentvisualactors (Variables|HorrorAction|GetDependentVisualActors))
  (if (Utilities|Array|IsNotEmpty _dependentvisualactors)
    (for _array_element _dependentvisualactors
      (Rendering|SetActorHiddenInGame _array_element false))
    (CallFunction|StoptheHorrorEvent (Variables|Default|GetEventDuration))))

(fn OnEventStop
  (bind _dependentvisualactors (Variables|HorrorAction|GetDependentVisualActors))
  (if (Utilities|Array|IsNotEmpty _dependentvisualactors)
    (for _array_element _dependentvisualactors
      (Rendering|SetActorHiddenInGame _array_element true))))