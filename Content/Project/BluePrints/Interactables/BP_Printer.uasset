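; BP_Printer is an interactable office copier that duplicates a paper the first-person player places in it.
; A state machine cycles from empty through ready, working, retrieve original and retrieve copy, driving the prompt text and interaction rules.
; Copying plays audio for a timed delay, spawns a BP_Paper with the original's mesh ID but another paper type, and reports progress to BP_TaskManager.
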(event Custom|Make%20Copy
  (bind _audio (Variables|Default|GetAudio))
  ;[1 1 1] make copy
  (if (Utilities|Enum|Equal(Enum) (Variables|Printer|GetState) "NewEnumerator1")
    (Variables|Printer|SetState "NewEnumerator2")
    (CallFunction|UpdatePreviewText)
    (Audio|Components|Audio|Play _audio 0.0)
    (Utilities|FlowControl|Delay (Variables|Printer|GetWork%20Time))
    (Variables|Printer|SetState "NewEnumerator4")
    (CallFunction|UpdatePreviewText)
    (Audio|Components|Audio|Stop _audio)
    (bind _asbp_paper (Utilities|Casting|CastToBP_Paper (Variables|Printer|GetscanSlotActor)))
    (bind _returnvalue (Game|SpawnActorfromClass "/Game/Project/BluePrints/BP_Paper.BP_Paper_C" (Transformation|GetWorldTransform (Variables|Default|GetCopySlot)) "AlwaysSpawn" "MultiplyWithRoot" 0 "NewEnumerator1" (Variables|/Game/Project/BluePrints/BP_Paper.BP_Paper_C|GetPaperMeshID _asbp_paper) 0))
    (Variables|Printer|SetcopySlotActor _returnvalue)
    (Utilities|IsValid (Variables|Default|GetTask%20Manager)
      (:Is%20Valid
        _)
      (:Is%20Not%20Valid
        (bind _returnvalue_2 (Actor|GetActorOfClass "/Game/Project/BluePrints/BP_TaskManager.BP_TaskManager_C"))
        (Variables|Default|SetTask%20Manager _returnvalue_2)))
    (Default|UpdateProgress (Variables|Default|GetTask%20Manager) "#000002" 1)))

(event EventBeginPlay
  (CallFunction|UpdatePreviewText))

(fn ConstructionScript
  (|CallParentFunction))

(fn UpdatePreviewText
  (switch Utilities|FlowControl|Switch|SwitchonE_Printer (Variables|Printer|GetState)
    (:NewEnumerator0
      (Variables|Default|SetPreviewText "put in the sheet")
      (Variables|Default|SetIsInteractable true :!label _label))
    (:NewEnumerator1
      (Variables|Default|SetPreviewText "start printer")
      (goto _label))
    (:NewEnumerator2
      (Variables|Default|SetIsInteractable false))
    (:NewEnumerator4
      (Variables|Default|SetPreviewText "retrive original")
      (goto _label))
    (:NewEnumerator3
      (Variables|Default|SetPreviewText "retrive copy")
      (goto _label))))

(fn TriggerInteraction
  (params (actor :type Actor%20Object%20Reference))
  (bind _asbp_player_1p (Utilities|Casting|CastToBP_Player1P actor))
  (switch Utilities|FlowControl|Switch|SwitchonE_Printer (Variables|Printer|GetState)
    (:NewEnumerator0
      (Variables|Printer|SetState "NewEnumerator1")
      (bind _actorinhand (Default|EmptyHand _asbp_player_1p))
      (bind _output_get (Variables|Printer|SetscanSlotActor _actorinhand))
      (Transformation|AttachComponentToComponent _output_get (Variables|Default|GetScanSlot) "None" "SnapToTarget" "SnapToTarget" "KeepRelative" false)
      (CallFunction|UpdatePreviewText :!label _label))
    (:NewEnumerator1
      (CallFunction|MakeCopy))
    (:NewEnumerator4
      (Variables|Printer|SetState "NewEnumerator3")
      (Default|PickUpinHand _asbp_player_1p (Variables|Printer|GetscanSlotActor))
      (Variables|Printer|SetscanSlotActor 0)
      (goto _label))
    (:NewEnumerator3
      (Variables|Printer|SetState "NewEnumerator0")
      (Default|PickUpinHand _asbp_player_1p (Variables|Printer|GetcopySlotActor))
      (Variables|Printer|SetcopySlotActor 0)
      (goto _label))))

(fn InteractCondition
  (params (actor :type Actor%20Object%20Reference))
  (bind _condition (|CallParentFunction actor))
  (bind _asbp_player_1p (Utilities|Casting|CastToBP_Player1P actor)
    (:then
      (switch Utilities|FlowControl|Switch|SwitchonE_Printer (Variables|Printer|GetState)
        (:NewEnumerator0
          (if (and _condition (Variables|/Game/Project/BluePrints/BP_Player1P.BP_Player1P_C|GetHasItemInHand _asbp_player_1p))
            (bind _asbp_paper (Utilities|Casting|CastToBP_Paper (Variables|/Game/Project/BluePrints/BP_Player1P.BP_Player1P_C|GetActorInHand _asbp_player_1p))
              (:then
                (return (Utilities|Enum|Equal(Enum) (Variables|/Game/Project/BluePrints/BP_Paper.BP_Paper_C|GetPaperType _asbp_paper) "NewEnumerator0")))
              (:CastFailed
                _)))
          (return false))
        (:NewEnumerator1
          (return _condition))
        (:NewEnumerator4
          _)
        (:NewEnumerator3
          _))
      (return (and _condition (not (Variables|/Game/Project/BluePrints/BP_Player1P.BP_Player1P_C|GetHasItemInHand _asbp_player_1p)))))
    (:CastFailed
      (return false))))