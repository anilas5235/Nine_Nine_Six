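; BP_PaperStack is an interactable stack that gives or takes paper from the first-person player, according to its access type.
; Pull spawns a BP_Paper of the stack's type with a random mesh into an empty hand, and Push destroys the held item.
; InteractCondition allows Push only for matching paper.
; TriggerInteraction also handles Push&Pull by choosing on hand state, though InteractCondition has no branch for it.
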(fn ConstructionScript
  (|CallParentFunction))

(fn InteractCondition
  (params (actor :type Actor%20Object%20Reference))
  (bind _condition (|CallParentFunction actor))
  (bind _asbp_player_1p (Utilities|Casting|CastToBP_Player1P actor)
    (:then
      (switch Utilities|FlowControl|Switch|SwitchonE_Accsess (Variables|PaperStack|GetAccsessType)
        (:NewEnumerator0
          (return (and _condition (not (Variables|/Game/Project/BluePrints/BP_Player1P.BP_Player1P_C|GetHasItemInHand _asbp_player_1p)))))
        (:NewEnumerator1
          (if (and _condition (Variables|/Game/Project/BluePrints/BP_Player1P.BP_Player1P_C|GetHasItemInHand _asbp_player_1p))
            (bind _asbp_paper (Utilities|Casting|CastToBP_Paper (Variables|/Game/Project/BluePrints/BP_Player1P.BP_Player1P_C|GetActorInHand _asbp_player_1p))
              (:then
                (return (Utilities|Enum|Equal(Enum) (Variables|/Game/Project/BluePrints/BP_Paper.BP_Paper_C|GetPaperType _asbp_paper) (Variables|PaperStack|GetPaperType))))
              (:CastFailed
                _)))
          (return false))))
    (:CastFailed
      (return false))))

(fn TriggerInteraction
  (params (actor :type Actor%20Object%20Reference))
  (switch Utilities|FlowControl|Switch|SwitchonE_Accsess (Variables|PaperStack|GetAccsessType)
    (:NewEnumerator0
      ;[1 1 1] Pull
      (bind _asbp_player_1p (Utilities|Casting|CastToBP_Player1P actor :!label _label))
      (if (not (Variables|/Game/Project/BluePrints/BP_Player1P.BP_Player1P_C|GetHasItemInHand _asbp_player_1p))
        (bind _returnvalue (Game|SpawnActorfromClass "/Game/Project/BluePrints/BP_Paper.BP_Paper_C" (Transformation|GetActorTransform _asbp_player_1p) "AlwaysSpawn" "MultiplyWithRoot" 0 (Variables|PaperStack|GetPaperType) (Math|Conversions|ToByte(Integer) (Math|Random|RandomIntegerinRange 0 5)) 0))
        (Default|PickUpinHand _asbp_player_1p _returnvalue)
        (Audio|PlaySound2D "/Game/Project/Audio/Tracs/MoreSoundsLib/Paper___Stationery/PaperPick.PaperPick" 1.0 1.0 0.0 0 0)))
    (:NewEnumerator1
      ;[1 1 1] Push
      (bind _asbp_player_1p_2 (Utilities|Casting|CastToBP_Player1P actor :!label _label_2))
      (if (Variables|/Game/Project/BluePrints/BP_Player1P.BP_Player1P_C|GetHasItemInHand _asbp_player_1p_2)
        (bind _actorinhand (Default|EmptyHand _asbp_player_1p_2))
        (Actor|DestroyActor _actorinhand)
        (Audio|PlaySound2D "/Game/Project/Audio/Tracs/MoreSoundsLib/Paper___Stationery/PaperPick.PaperPick" 1.0 1.0 0.0 0 0)))
    (:NewEnumerator2
      (bind _asbp_player_1p_3 (Utilities|Casting|CastToBP_Player1P actor))
      (if (Variables|/Game/Project/BluePrints/BP_Player1P.BP_Player1P_C|GetHasItemInHand _asbp_player_1p_3)
        (goto _label_2)
        (else
          (goto _label))))))