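; BP_Door is an interactable door that opens on first interaction and calls PossessCam on later ones.
; TriggerInteraction branches on IsOpen, and OpenDoor sets that flag, applies an instant 30-degree yaw rotation to the door mesh and plays a creak sound.
; PreviewText starts as CloseDoorText and switches to OpenDoorText when opened, with no path to close the door again.
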(event EventBeginPlay
  (Variables|Default|SetPreviewText (Variables|Door|GetCloseDoorText)))

(fn ConstructionScript)

(fn OpenDoor
  (Variables|Door|SetIsOpen true)
  (Variables|Default|SetPreviewText (Variables|Door|GetOpenDoorText))
  (Transformation|AddWorldRotation (Variables|Default|GetSM_Door) "0.000000,30.000000,0.000000" false false)
  (Audio|PlaySoundatLocation "/Game/Project/Audio/Tracs/SFX/Door/door-open-with-a-creak_Cue.door-open-with-a-creak_Cue" (Transformation|GetActorLocation) "0, 0, 0" 1.0 1.0 0.0 0 0 0 0)
  (return))

(fn TriggerInteraction
  (params (actor :type Actor%20Object%20Reference))
  (if (Variables|Door|GetIsOpen)
    (CallFunction|PossessCam)
    (else
      (CallFunction|OpenDoor))))