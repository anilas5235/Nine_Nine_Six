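; Interactable coffee machine that brews a cup and, when taken, resets the coffee level on the PC996 actor.
; A state enum cycles Idle, Working and CoffeeReady: interacting starts a timed brew with looping-style audio, then reveals the cup mesh for pickup.
; Each state change refreshes the interaction prompt text and disables interaction while brewing.
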(event Custom|MakeCoffee
  (bind _audio (Variables|Default|GetAudio))
  ;[1 1 1] Make Coffee
  (if (Utilities|Enum|Equal(Enum) (Variables|Coffee_Machine|GetState) "NewEnumerator2")
    (Variables|Coffee_Machine|SetState "NewEnumerator1")
    (CallFunction|UpdatePreviewText)
    (Audio|Components|Audio|Play _audio 0.0)
    (Utilities|FlowControl|Delay (Variables|CoffeeMachine|GetWorkTime))
    (Variables|Coffee_Machine|SetState "NewEnumerator0")
    (CallFunction|UpdatePreviewText)
    (Audio|Components|Audio|Stop _audio)
    (Development|SetHiddeninGame (Variables|Default|GetcoffeeCup) false false)))

(event Custom|Take%20Coffee
  ;[1 1 1] Take Coffee
  (Variables|Coffee_Machine|SetState "NewEnumerator2")
  (CallFunction|UpdatePreviewText)
  (bind _aspc_996 (CallFunction|TryGetPC996))
  (Default|ResetCoffeeLevel _aspc_996)
  (Development|SetHiddeninGame (Variables|Default|GetcoffeeCup) true false))

(event EventBeginPlay
  ;[1 1 1] Begin
  (CallFunction|UpdatePreviewText)
  (Development|SetHiddeninGame (Variables|Default|GetcoffeeCup) true false))

(fn ConstructionScript
  (|CallParentFunction))

(fn UpdatePreviewText
  (switch Utilities|FlowControl|Switch|SwitchonE_CoffeMachine (Variables|Coffee_Machine|GetState)
    (:NewEnumerator2
      (Variables|Default|SetPreviewText (Variables|CoffeeMachine|GetTextWithoutCoffee))
      (Variables|Default|SetIsInteractable true :!label _label))
    (:NewEnumerator0
      (Variables|Default|SetPreviewText (Variables|CoffeeMachine|GetTextWithCoffee))
      (goto _label))
    (:NewEnumerator1
      (Variables|Default|SetIsInteractable false))))

(fn TriggerInteraction
  (params (actor :type Actor%20Object%20Reference))
  (switch Utilities|FlowControl|Switch|SwitchonE_CoffeMachine (Variables|Coffee_Machine|GetState)
    (:NewEnumerator2
      (CallFunction|MakeCoffee))
    (:NewEnumerator0
      (CallFunction|TakeCoffee))))